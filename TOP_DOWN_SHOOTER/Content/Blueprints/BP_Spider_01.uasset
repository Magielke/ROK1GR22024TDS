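; BP_Spider_01 is an enemy spider that chases the player and attacks in melee.
; A looping AI MoveTo drives the chase, while Tick pauses movement to play the attack montage within range.
; AnyDamage lowers health and sets the dead flag at zero, but every hit also disables movement and collision, calls PlayMontage with no montage set, and destroys the spider after a delay.
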(event `self.ReceiveBeginPlay`
  (if (`self.IsAlive`)
    (`|AIMoveTo` self (0.0 0.0 0.0) (`GameplayStatics.GetPlayerCharacter` 0) :!label _label
      (:`OnSuccess`
        (`KismetSystemLibrary.Delay` 0.2)
        (goto _label)))))

(event `self.ReceiveTick`
  (params (DeltaSeconds :type "Float (single-precision)"))
  ;[1 0.3236 0.4335] AttackAnim
  (if (and (`self.IsAttackRange`) (not (`self.IsAttacking`)))
    (if (`self.IsAlive`)
      (`ActorComponent.Deactivate` (`self.CharacterMovement`))
      (`|PlayMontage` (`self.Mesh`) "/Game/Characters/Enemy_Great_Spider/Animations/AM_SpiderAttack.AM_SpiderAttack"
        (:`OnCompleted`
          (`ActorComponent.Activate` (`self.CharacterMovement`) false))))))

(event `self.ReceiveAnyDamage`
  (params (Damage :type "Float (single-precision)") (DamageType :type "DamageType Object Reference") (InstigatedBy :type "Controller Object Reference") (DamageCauser :type "Actor Object Reference"))
  ;[1 0.04688 0.04688] Dead
  (bind _output_get (set `self.Health` (`KismetMathLibrary.FClamp` (- (`self.Health`) Damage) 0.0 100.0)))
  (`self.Kill Spider` (== _output_get 0.0))
  (`|PlayMontage` (`self.Mesh`)
    (:`then`
      (`KismetSystemLibrary.Delay` 5.0)
      (`self.K2_DestroyActor`))))

(fn `IsAlive`
  (returns (ReturnValue :type Boolean))
  (return (not (`self.Dead`))))

(fn `IsAttacking`
  (returns (ReturnValue :type Boolean))
  (return (`AnimInstance.Montage_IsPlaying` (`SkeletalMeshComponent.GetAnimInstance` (`self.Mesh`)) null)))

(fn `IsAttackRange`
  (returns (ReturnValue :type Boolean))
  (return (< (`self.GetDistanceTo` (`GameplayStatics.GetPlayerCharacter` 0)) (`self.AttackRange`))))

(fn `Kill Spider`
  (params (Dead :type Boolean))
  (set `self.Dead` Dead)
  (`ActorComponent.Deactivate` (`self.CharacterMovement`))
  (`self.SetActorEnableCollision` false))

(fn `UserConstructionScript`)