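; Player character Blueprint with movement, automatic rifle fire, health and death, which creates its HUD widget on BeginPlay.
; While alive, it moves along the controller's axes and eases control yaw toward the direction of mouse movement above a dead zone.
; Holding Fire runs muzzle effects, looping sound and a timer-repeated line trace from the weapon socket that applies damage.
; Incoming damage reduces clamped health, setting Dead at zero and stopping fire effects.
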(event `self.ReceiveTick`
  (params (DeltaSeconds :type "Float (single-precision)"))
  ;[0.16 0.2613 1] Movement
  (if (`self.IsAlive`)
    (`self.Update_Char_Rotation`)))

(event `InputAxis|Move_Forward_Back`
  (params (AxisValue :type "Float (single-precision)"))
  ;[0.16 0.2613 1] Movement
  (if (`self.IsAlive`)
    (`self.AddMovementInput` (`self.GetActorForwardVector` (`GameplayStatics.GetPlayerController` 0)) AxisValue)))

(event `InputAxis|Move_Left_Right`
  (params (AxisValue :type "Float (single-precision)"))
  ;[0.16 0.2613 1] Movement
  (if (`self.IsAlive`)
    (`self.AddMovementInput` (`self.GetActorRightVector` (`GameplayStatics.GetPlayerController` 0)) AxisValue)))

(event `InputAction|Fire`
  (params (Key :type "Key Structure"))
  ;[1 0.685 0.1293] Shooting
  (:`Pressed`
    (if (`self.IsAlive`)
      (`self.StartFired`)
      (`self.WeaponTrace`)
      (`KismetSystemLibrary.K2_SetTimer` null "Weapon Trace" 0.08 true)))
  (:`Released`
    (`self.StopFired`)
    (if (`self.IsAlive`)
      (`GameplayStatics.SpawnSound2D` "/Game/Sounds/Weapon_AssaultRifle/Stereo/SC_End.SC_End" 1.0 1.0 0.0 null)
      (`KismetSystemLibrary.K2_ClearTimer` null "Weapon Trace"))))

(event `self.ReceiveBeginPlay`
  ;[1 1 1] UI
  (bind _returnvalue (`|CreateWidget` "/Game/UI/W_PlayerHUD_01.W_PlayerHUD_01_C" null self))
  (`UserWidget.AddToViewport` _returnvalue 0))

(event `self.ReceiveAnyDamage`
  (params (Damage :type "Float (single-precision)") (DamageType :type "DamageType Object Reference") (InstigatedBy :type "Controller Object Reference") (DamageCauser :type "Actor Object Reference"))
  ;[1 0.04688 0.04688] Dead
  (bind _output_get (set `self.Health` (`KismetMathLibrary.FClamp` (- (`self.Health`) Damage) 0.0 100.0)))
  (bind _output_get_2 (set `self.Dead` (== _output_get 0.0)))
  (if _output_get_2
    (`self.StopFired`)))

(fn `Add Health`
  (params (`Health to add` :type "Float (double-precision)"))
  (set `self.Health` (`KismetMathLibrary.FClamp` (+ (`self.Health`) `Health to add`) 0.0 100.0)))

(fn `GetEndLocationLT`
  (returns (ReturnValue :type "Vector Structure"))
  (return (+ (`self.GetStartLocartionLT`) (* (`KismetMathLibrary.GetForwardVector` (`self.GetControlRotation`)) (`self.WeaponRange`)))))

(fn `GetStartLocartionLT`
  (returns (ReturnValue :type "Vector Structure"))
  (return (`SceneComponent.GetSocketLocation` (`self.Weapon`) "P_AssaultRifle_MF")))

(fn `Is Health Full`
  (returns (ReturnValue :type Boolean))
  (return (== (`self.Health`) 100.0)))

(fn `Is_Move_Above_Dead_Zone`
  (returns (ReturnValue :type Boolean))
  (return (> (`KismetMathLibrary.VSize2D` (`self.MouseVelocity`)) (`self.Dead Zone`))))

(fn `IsAlive`
  (returns (ReturnValue :type Boolean))
  (return (not (`self.Dead`))))

(fn `MouseVelocity`
  (returns (ReturnValue :type "Vector2D Structure"))
  (bind (_deltax _deltay) (`PlayerController.GetInputMouseDelta` (`GameplayStatics.GetPlayerController` 0)))
  (return (/ (`KismetMathLibrary.MakeVector2D` _deltax _deltay) (`GameplayStatics.GetWorldDeltaSeconds`))))

(fn `StartFired`
  (`ActorComponent.Activate` (`self.P_AssaultRifle_MF`) false)
  (bind _returnvalue (`GameplayStatics.SpawnSound2D` "/Game/Sounds/Weapon_AssaultRifle/Stereo/SC_WeaponFired_01.SC_WeaponFired_01" 1.0 1.0 0.0 null))
  (set `self.WeaponSound` _returnvalue))

(fn `StopFired`
  (bind _weaponsound (`self.WeaponSound`))
  (`ActorComponent.Deactivate` (`self.P_AssaultRifle_MF`))
  (`/Engine/EditorBlueprintResources/StandardMacros.IsValid` _weaponsound
    (:`Is Valid`
      (`AudioComponent.Stop` _weaponsound))))

(fn `Update_Char_Rotation`
  (bind _returnvalue (`GameplayStatics.GetPlayerController` 0))
  (bind (_returnvalue_x _returnvalue_y) (`KismetMathLibrary.BreakVector2D` (`self.MouseVelocity`)))
  (if (`self.Is_Move_Above_Dead_Zone`)
    (`Controller.SetControlRotation` _returnvalue (`KismetMathLibrary.RInterpTo` (`Controller.GetControlRotation` _returnvalue) (`KismetMathLibrary.MakeRotator` 0.0 0.0 (`KismetMathLibrary.DegAtan2` _returnvalue_x _returnvalue_y)) (`GameplayStatics.GetWorldDeltaSeconds`) (`self.Interp Speed`)))))

(fn `UserConstructionScript`)

(fn `WeaponTrace`
  (bind _outhit (`KismetSystemLibrary.LineTraceSingle` :`Start` (`self.GetStartLocartionLT`) :`End` (`self.GetEndLocationLT`) :`TraceChannel` "TraceTypeQuery1" :`DrawDebugType` "ForDuration"))
  (`GameplayStatics.ApplyDamage` (`.HitActor` (`GameplayStatics.BreakHitResult` _outhit)) (`self.DamagePerHit`)))